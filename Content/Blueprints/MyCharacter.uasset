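; Character Blueprint for melee-style directional attacks, with left mouse switching on offense mode.
; CombatModeAttack updates a first-click flag, then plays the "Offense_" montage section matching the Direction value.
; A forward attack also calls ChargeAttack, which nav-raycasts along the player pawn's velocity and moves to the hit point.
; That move only runs if the pawn's controller casts to AIController.
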(event Input|MouseEvents|LeftMouseButton
  (:Pressed
    (Variables|Default|SetIsOffenseMode true)))

(fn ConstructionScript)

(fn CombatModeAttack
  (if (Math|Boolean|Equal(Boolean) (Variables|Default|GetIsOffenseMode) true)
    (LocalVariables|SetOffenseNFirstClick false)
    (else
      (LocalVariables|SetOffenseNFirstClick true)))
  (CallFunction|PlayAttackAnimation))

(fn PlayAttackAnimation
  (switch int (Variables|Default|GetDirection)
    (:Default
      (LocalVariables|SetNewLocalVar_0 "Default"))
    (:0
      (LocalVariables|SetNewLocalVar_0 "Left"))
    (:1
      (LocalVariables|SetNewLocalVar_0 "Right"))
    (:2
      (LocalVariables|SetNewLocalVar_0 "Fwd"))
    (:3
      (LocalVariables|SetNewLocalVar_0 "Back")))
  (if true
    (Animation|PlayAnimMontage 0 1.0 (Utilities|String|StringToName (Utilities|String|Append "Offense_" (LocalVariables|GetNewLocalVar_0))))
    (if (Utilities|Enum|Equal(Enum) (LocalVariables|GetNewLocalVar_0) "Fwd")
      (CallFunction|ChargeAttack (Game|Player|GetPlayerPawn 0)))))

(fn ChargeAttack
  (params (Target :type Actor%20Object%20Reference))
  (bind _returnvalue (Game|Player|GetPlayerPawn 0))
  (bind _returnvalue_2 (Transformation|GetActorLocation _returnvalue))
  (bind _hitlocation (Class|NavigationSystem|NavigationRaycast _returnvalue_2 (+ _returnvalue_2 (* (Math|Vector|Normalize (Transformation|GetVelocity _returnvalue)) 1e+04))))
  (bind _asaicontroller (Utilities|Casting|CastToAIController (Pawn|GetController _returnvalue)))
  (AI|Navigation|MovetoLocation _asaicontroller _hitlocation -1.0 true true false false))